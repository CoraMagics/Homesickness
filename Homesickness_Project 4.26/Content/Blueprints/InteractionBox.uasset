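; InteractionBox is a chainable VR task trigger that shows an exclamation-mark mesh while activated.
; Motion controller overlap on an active box enables input, so GrabRight fires once.
; It either broadcasts StartMinigame or plays a fade-out cutscene with sound, then advances and broadcasts TaskDone.
; Advancing disables input and hands activation and marker visibility to NextInteractionBox, or opens LevelName when none is valid.
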(event OnComponentBeginOverlap(Box)
  (params (OverlappedComponent :type Primitive%20Component%20Object%20Reference) (OtherActor :type Actor%20Object%20Reference) (OtherComp :type Primitive%20Component%20Object%20Reference) (OtherBodyIndex :type Integer) (bFromSweep :type Boolean) (SweepResult :type Hit%20Result%20Structure%20%28by%20ref%29))
  ;[1 1 1] Enables input
  (Utilities|Casting|CastToBP_MotionController OtherActor)
  (if (Variables|Default|GetActivated)
    (Input|EnableInput (Game|GetPlayerController 0))))

(event Custom|ActivateNextInteractionBox
  (bind _nextinteractionbox (Variables|Default|GetNextInteractionBox))
  ;[1 1 1] Disables input + Sets up new interactionBox
  (Input|DisableInput (Game|GetPlayerController 0))
  (Utilities|IsValid _nextinteractionbox
    (:Is%20Valid
      (Variables|InteractionBox_C|SetActivated _nextinteractionbox true)
      (CallFunction|MakeVisible _nextinteractionbox)
      (Variables|Default|SetActivated false)
      (CallFunction|MakeVisible))
    (:Is%20Not%20Valid
      (Game|OpenLevel(byName) (Variables|Default|GetLevel%20Name)))))

(event Custom|MakeVisible
  (bind _staticmesh (Variables|Default|GetStaticMesh))
  ;[1 1 1] Exclamation Mark
  (if (Variables|Default|GetActivated)
    (Development|SetHiddeninGame _staticmesh false false)
    (Rendering|SetVisibility _staticmesh true false)
    (else
      (Development|SetHiddeninGame _staticmesh true false)
      (Rendering|SetVisibility _staticmesh false false))))

(event Input|ActionEvents|InputActionGrabRight
  (params (Key :type Key%20Structure :default "None"))
  ;[1 1 1] Cutscene
  (:Pressed
    (Utilities|FlowControl|DoOnce false
      (:Completed
        (if (Variables|Default|GetHas_Minigame)
          (Default|CallStartMinigame)
          (else
            (CameraFades|StartCameraFade :self (Game|GetPlayerCameraManager 0) :ToAlpha 1.0 :Duration 1.5 :bHoldWhenFinished true)
            (Utilities|FlowControl|Delay 1.5)
            (Audio|PlaySound2D (Variables|Default|GetInteractionSound) 1.0 1.0 0.0 0 0)
            (Utilities|FlowControl|Delay (Variables|Default|GetDuration))
            (CameraFades|StartCameraFade :self (Game|GetPlayerCameraManager 0) :FromAlpha 1.0 :Duration 1.5 :bHoldWhenFinished true)
            (CallFunction|ActivateNextInteractionBox)
            (Default|CallTaskDone)))))))

(fn ConstructionScript
  (bind _staticmesh (Variables|Default|GetStaticMesh))
  (if (Variables|Default|GetActivated)
    (Development|SetHiddeninGame _staticmesh false false)
    (Rendering|SetVisibility _staticmesh true false)
    (else
      (Development|SetHiddeninGame _staticmesh true false)
      (Rendering|SetVisibility _staticmesh false false))))