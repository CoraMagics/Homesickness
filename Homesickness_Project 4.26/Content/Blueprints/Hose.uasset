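; Hose is an interactable actor that triggers a one-time blackout-and-explosion sequence when the player grabs it with a VR motion controller.
; Overlapping its Box with a BP_MotionController enables input, which is never disabled afterward.
; The first GrabRight press then fades the camera out, plays an explosion sound, and fades back in after a delay.
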(event OnComponentBeginOverlap(Box)
  (params (OverlappedComponent :type Primitive%20Component%20Object%20Reference) (OtherActor :type Actor%20Object%20Reference) (OtherComp :type Primitive%20Component%20Object%20Reference) (OtherBodyIndex :type Integer) (bFromSweep :type Boolean) (SweepResult :type Hit%20Result%20Structure%20%28by%20ref%29))
  (Utilities|Casting|CastToBP_MotionController OtherActor)
  (Input|EnableInput (Game|GetPlayerController 0)))

(event EventBeginPlay)

(event Collision|EventActorBeginOverlap
  (params (OtherActor :type Actor%20Object%20Reference)))

(event EventTick
  (params (DeltaSeconds :type Float%20%28single-precision%29)))

(event Input|ActionEvents|InputActionGrabRight
  (params (Key :type Key%20Structure :default "None"))
  (:Pressed
    (Utilities|FlowControl|DoOnce false
      (:Completed
        (CameraFades|StartCameraFade :self (Game|GetPlayerCameraManager 0) :ToAlpha 1.0 :Duration 1.5 :bHoldWhenFinished true)
        (Utilities|FlowControl|Delay 1.5)
        (Audio|PlaySound2D "/Game/StarterContent/Audio/Explosion01.Explosion01" 1.0 1.0 0.0 0 0)
        (Utilities|FlowControl|Delay 1e+01)
        (CameraFades|StartCameraFade :self (Game|GetPlayerCameraManager 0) :FromAlpha 1.0 :Duration 1.5 :bHoldWhenFinished true)))))

(fn ConstructionScript)